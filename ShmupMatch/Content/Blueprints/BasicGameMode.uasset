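; Game mode that runs data-table-driven waves of enemy ships.
; StartGame gathers all SpawnPoint actors, loads the row names of FirstLevelSpawnTable as waves and starts a timer on SpawnObject.
; SpawnObject has the row's chosen spawn point create an EnemyShip, optionally on a spline, applies its stats, then re-arms a one-shot timer using the row's delays within and between waves.
; DestroySpawnedActors clears the SpawnedActors list, destroying each actor.
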(event Custom|Start%20Game
  (CallFunction|FetchSpawnPoints)
  (Variables|Default|SetIs%20Spawning true)
  (Utilities|Time|SetTimerbyEvent (delegate Custom|Spawn%20Object) 1.0)
  (bind _outrownames (DataTable|GetDataTableRowNames "/Game/Blueprints/FirstLevelSpawnTable.FirstLevelSpawnTable"))
  (Variables|Default|SetWaves%20To%20Spawn _outrownames))

(event Custom|Destroy%20Spawned%20Actors
  (bind _spawned_actors (Variables|Default|GetSpawned%20Actors))
  (for _array_element _spawned_actors
    (Actor|DestroyActor _array_element))
  (Utilities|Array|Clear _spawned_actors))

(event Custom|Fetch%20Spawn%20Points
  (Utilities|Array|Clear (Variables|Default|GetSpawn%20Points))
  (bind _outactors (Actor|GetAllActorsOfClass "/Game/Blueprints/SpawnPoint.SpawnPoint_C"))
  (Variables|Default|SetSpawn%20Points _outactors))

(event Custom|Spawn%20Object
  (bind _current_wave (Variables|Default|GetCurrent%20Wave))
  (bind _returnvalue (Utilities|GetDataTableRow "/Game/Blueprints/FirstLevelSpawnTable.FirstLevelSpawnTable" (Utilities|Array|Get(acopy) (Variables|Default|GetWaves%20To%20Spawn) (Variables|Default|GetCurrent%20Wave)))
    (:then
      (bind _spawned_actor (Default|SpawnObject (Utilities|Array|Get(acopy) (Variables|Default|GetSpawn%20Points) (.SpawnPointToUse (Utilities|Struct|BreakSpawnData _returnvalue))) "/Game/Blueprints/EnemyShip.EnemyShip_C" (.UsesSplineForMovement (Utilities|Struct|BreakSpawnData _returnvalue))))
      (bind _asenemy_ship (Utilities|Casting|CastToEnemyShip _spawned_actor))
      (Default|SetupStats _asenemy_ship (.EnemyShip (Utilities|Struct|BreakSpawnData _returnvalue)))
      (if (== (Variables|Default|GetCurrent%20Spawn) (- (.NumberToSpawn (Utilities|Struct|BreakSpawnData _returnvalue)) 1))
        (Variables|Default|SetCurrent%20Spawn 0)
        (Math|Integer|IncrementInt _current_wave
          (:%20%20
            (if (not (> _current_wave (Utilities|Array|Length (Variables|Default|GetWaves%20To%20Spawn))))
              (Utilities|Time|SetTimerbyEvent (delegate Custom|Spawn%20Object) (.TimeUntilNextSpawn (Utilities|Struct|BreakSpawnData _returnvalue))))))
        (else
          (Math|Integer|IncrementInt (Variables|Default|GetCurrent%20Spawn)
            (:%20%20
              (Utilities|Time|SetTimerbyEvent (delegate Custom|Spawn%20Object) (.TimeBetweenSpawnsForThisRow (Utilities|Struct|BreakSpawnData _returnvalue))))))))))

(event EventBeginPlay)

(event EventTick
  (params (DeltaSeconds :type Float%20%28single-precision%29)))

(fn ConstructionScript)