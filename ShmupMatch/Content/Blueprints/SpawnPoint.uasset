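; SpawnPoint is a placeable spawner that creates enemy ships for the game at its Billboard component's transform.
; Its SpawnObject function spawns a given actor class, always ignoring collision, and casts it to EnemyShip.
; The ship then either follows the point's Spline or takes its movement direction from the Direction component's forward vector, depending on a flag.
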(event EventBeginPlay)

(fn ConstructionScript)

(fn SpawnObject
  (params (Actor%20To%20Spawn :type Actor%20Class%20Reference) (Jump%20On%20Spline? :type Boolean))
  (bind _returnvalue (Game|SpawnActorfromClass Actor%20To%20Spawn (Transformation|GetWorldTransform (Variables|Default|GetBillboard)) "AlwaysSpawn" 0 0))
  (bind _asenemy_ship (Utilities|Casting|CastToEnemyShip _returnvalue))
  (if Jump%20On%20Spline?
    (Default|UseSpline _asenemy_ship (Variables|Default|GetSpline))
    (else
      (Variables|/Game/Blueprints/EnemyShip.EnemyShip_C|SetDirection _asenemy_ship (Math|Vector|GetForwardVector (Variables|Default|GetDirection)))))
  (return _returnvalue))