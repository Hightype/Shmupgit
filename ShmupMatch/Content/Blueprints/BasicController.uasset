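; BasicController is a controller that relays player input to the SpaceshipPawn.
; On BeginPlay it casts player pawn 0 to SpaceshipPawn and caches the reference.
; The Right and Down axes drive the ship's X and Y movement functions, and pressing Fire calls its FireProjectile, leaving movement and firing logic to the pawn.
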(event Custom|Setup%20Spaceship%20Pawn
  (bind _asspaceship_pawn (Utilities|Casting|CastToSpaceshipPawn (Game|Player|GetPlayerPawn 0)))
  (Variables|Default|SetSpaceship _asspaceship_pawn))

(event EventBeginPlay
  (CallFunction|SetupSpaceshipPawn))

(event Input|ActionEvents|InputActionFire
  (params (Key :type Key%20Structure))
  (:Pressed
    (Default|FireProjectile (Variables|Default|GetSpaceship))))

(event Input|AxisEvents|InputAxisDown
  (params (AxisValue :type Float%20%28single-precision%29))
  (Default|MoveYAxis (Variables|Default|GetSpaceship) AxisValue))

(event Input|AxisEvents|InputAxisRight
  (params (AxisValue :type Float%20%28single-precision%29))
  (Default|MoveXAxis (Variables|Default|GetSpaceship) AxisValue))

(fn ConstructionScript)