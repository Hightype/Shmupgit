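; EnemyShip is an enemy ship actor that takes its sprite and speed from a stats struct passed to SetupStats, which also starts movement.
; Each Tick it moves along Direction at that speed with a swept SetActorLocation, after BeginPlay fixes its rotation.
; UseSpline stores a spline and switches off directional movement, but no spline-following logic is implemented here.
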(event Custom|Use%20Spline
  (params (Spline%20To%20Use :type Spline%20Component%20Object%20Reference))
  (Variables|Default|SetSpline%20To%20Follow Spline%20To%20Use)
  (Variables|Default|SetIs%20Using%20Spline true))

(event Custom|Setup%20Stats
  (params (Stats :type Enemy%20Ship%20Data%20Structure))
  (bind _output_get (Variables|Default|SetEnemy%20Ship%20Data Stats))
  (Rendering|Components|Sprite|SetSprite (Variables|Default|GetPaperSprite) (.ShipTexture (Utilities|Struct|BreakEnemyShipData _output_get)))
  (Variables|Default|SetIs%20Moving true))

(event EventBeginPlay
  (Transformation|SetActorRotation "-90.000000,90.000000, 0"))

(event Collision|EventActorBeginOverlap
  (params (OtherActor :type Actor%20Object%20Reference)))

(event EventTick
  (params (DeltaSeconds :type Float%20%28single-precision%29))
  (if (Variables|Default|GetIs%20Moving)
    (if (not (Variables|Default|GetIs%20Using%20Spline))
      (Transformation|SetActorLocation (+ (* (* (Variables|Default|GetDirection) (.Speed (Utilities|Struct|BreakEnemyShipData (Variables|Default|GetEnemy%20Ship%20Data)))) DeltaSeconds) (Transformation|GetActorLocation)) true false))))

(fn ConstructionScript)