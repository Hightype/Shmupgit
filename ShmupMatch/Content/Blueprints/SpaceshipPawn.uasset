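; Player spaceship pawn, shown as a sprite that is rotated upright at BeginPlay and moved by two input axes.
; Axis events offset the sprite's world location along world right and up, then set it as the actor location, without delta-time scaling.
; Only vertical moves sweep for collision; horizontal moves do not.
; The FireProjectile event is an empty stub.
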(event Custom|Move%20X%20Axis
  (params (Axis :type Float%20%28single-precision%29))
  (Transformation|SetActorLocation (+ (* (Math|Vector|GetRightVector "0, 0, 0") Axis) (Transformation|GetWorldLocation (Variables|Default|GetSpaceship%20Sprite))) false false))

(event Custom|Fire%20Projectile)

(event Custom|Move%20Y%20Axis
  (params (Axis :type Float%20%28single-precision%29))
  (Transformation|SetActorLocation (+ (* (Math|Vector|GetUpVector "0, 0, 0") Axis) (Transformation|GetWorldLocation (Variables|Default|GetSpaceship%20Sprite))) true false))

(event EventBeginPlay
  (Transformation|SetWorldRotation (Variables|Default|GetSpaceship%20Sprite) "90.000000,90.000000,0.000000" false false))

(fn ConstructionScript)